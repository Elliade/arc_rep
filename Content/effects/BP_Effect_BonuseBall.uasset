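; BP_Effect_BonuseBall is an effect Blueprint, apparently a ball bonus meant to create a blast where its owner hits something.
; EffectStart binds to the owner's OnActorHit and EffectEnd unbinds, each calling its parent only when the owner is valid.
; GenerateBlast matches the hit signature and is the likely handler, but it only draws a temporary red debug sphere at the impact point, with no damage or force.
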(fn `EffectEnd`
  (bind _returnvalue (`self.GetOwner`))
  (`/Engine/EditorBlueprintResources/StandardMacros.IsValid` _returnvalue
    (:`Is Valid`
      (remove `Actor.OnActorHit` _returnvalue (`|CreateDelegate` :!event `GenerateBlast`))
      (`parent.EffectEnd`))))

(fn `EffectStart`
  (bind _returnvalue (`self.GetOwner`))
  (`/Engine/EditorBlueprintResources/StandardMacros.IsValid` _returnvalue
    (:`Is Valid`
      (add `Actor.OnActorHit` _returnvalue (`|CreateDelegate` :!event `GenerateBlast`))
      (`parent.EffectStart`))))

(fn `GenerateBlast`
  (params (SelfActor :type "Actor Object Reference") (OtherActor :type "Actor Object Reference") (NormalImpulse :type "Vector Structure") (Hit :type "HitResult Structure (by ref)"))
  (`KismetSystemLibrary.DrawDebugSphere` (`.Location` (`GameplayStatics.BreakHitResult` Hit)) 100.0 25 (struct :`R` 1.0 :`B` 0.00746 :`A` 1.0) 6.0)
  (return))