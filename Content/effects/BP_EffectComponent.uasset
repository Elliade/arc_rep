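; BP_EffectComponent is an effect component that manages a timed start and end, with no visible effect logic of its own.
; InitializeEffectComponent stores both delays and sets a one-shot timer for the start delay, presumably leading to EffectStart.
; EffectStart sets a second timer for the end delay, presumably leading to EffectEnd, which destroys the component.
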(fn `EffectEnd`
  (`self.K2_DestroyComponent`))

(fn `EffectStart`
  (`KismetSystemLibrary.K2_SetTimerDelegate` (`|CreateDelegate` :!event `EffectEnd`) (`self.Effect End Delay`)))

(fn `InitializeEffectComponent`
  (params (EffectStartDelay :type "Float (double-precision)") (EffectEndDelay :type "Float (double-precision)"))
  (locals (NewLocalVar :type "Float (double-precision)") (NewLocalVar_0 :type "Float (double-precision)"))
  (set `self.Effect Start Delay` EffectStartDelay)
  (set `self.Effect End Delay` EffectEndDelay)
  (`KismetSystemLibrary.K2_SetTimerDelegate` (`|CreateDelegate` :!event `EffectStart`) (`self.Effect Start Delay`)))