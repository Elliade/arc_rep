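; A bonus actor that, when activated, spawns an extra bonus ball for the player, despite its "WithEffect" name.
; Activate finds the BP_Plate actor, spawns a BP_BonuseBall at its Sphere's world location regardless of collision, then calls the parent Activate.
; An unconnected branch would attach a timed effect component of EffectClass to every BP_Ball, but it never runs.
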(fn `Activate`
  ;[1 1 1] Спаун доп мячика
  (bind _returnvalue (`GameplayStatics.GetActorOfClass` "/Game/Actors/BP_Plate.BP_Plate_C"))
  (`|SpawnActorFromClass` "/Game/Actors/BP_BonuseBall.BP_BonuseBall_C" (`KismetMathLibrary.MakeTransform` (`SceneComponent.K2_GetComponentLocation` (`/Game/Actors/BP_Plate.Sphere` _returnvalue))) "AlwaysSpawn" "MultiplyWithRoot" null null)
  (`parent.Activate`))

(fn `UserConstructionScript`
  (`parent.UserConstructionScript`))