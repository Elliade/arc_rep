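; BP_Block is a breakable block that takes damage from balls and can drop a bonus.
; On BeginPlay it gets random health from 1 to 3 in BPHealthComponent, binds health and death events, and colors its cube to match.
; Hits from BP_Ball or BP_BonuseBall subtract health.
; SetMaterial recolors the cube as health drops, while SpawnBonuse destroys the block and sometimes spawns BP_BonuseWithEffect.
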(event `self.ReceiveBeginPlay`
  (bind _bp_healthcomponent (`self.BP_HealthComponent`))
  (bind _cube (`self.Cube`))
  (bind _hp (`/Game/Actors/ActorComponents/BP_HealthComponent.HP` _bp_healthcomponent))
  ;[1 1 1] ХП и цвет блоков
  (set `/Game/Actors/ActorComponents/BP_HealthComponent.HP` (`KismetMathLibrary.RandomIntegerInRange` 1 3) _bp_healthcomponent)
  (`self.Binds`)
  (if (== _hp 3)
    (`PrimitiveComponent.SetMaterial` _cube 0 "/Game/Actors/Materials/Red.Red")
    (elif (== _hp 2)
      (`PrimitiveComponent.SetMaterial` _cube 0 "/Game/Actors/Materials/Yellow.Yellow")
      (else
        (`PrimitiveComponent.SetMaterial` _cube 0 "/Game/Actors/Materials/Green.Green")))))

(event `self.ReceiveHit`
  (params (MyComp :type "PrimitiveComponent Object Reference") (Other :type "Actor Object Reference") (OtherComp :type "PrimitiveComponent Object Reference") (bSelfMoved :type Boolean) (HitLocation :type "Vector Structure") (HitNormal :type "Vector Structure") (NormalImpulse :type "Vector Structure") (Hit :type "HitResult Structure (by ref)"))
  ;[1 1 1] Взаимодействие с мячиками
  (cast `/Game/Actors/BP_Ball` Other
    (:`then`
      _)
    (:`CastFailed`
      (cast `/Game/Actors/BP_BonuseBall` Other)))
  (`/Game/Actors/ActorComponents/BP_HealthComponent.Sub` (`self.BP_HealthComponent`)))

(fn `Binds`
  (bind _bp_healthcomponent (`self.BP_HealthComponent`))
  (add `/Game/Actors/ActorComponents/BP_HealthComponent.OnHealthUpdate` _bp_healthcomponent (`|CreateDelegate` :!event `Set Material`))
  (add `/Game/Actors/ActorComponents/BP_HealthComponent.OnDeath` _bp_healthcomponent (`|CreateDelegate` :!event `Spawn_Bonuse`)))

(fn `Set Material`
  (params (OldHealth :type Integer) (NewHealth :type Integer))
  (bind _cube (`self.Cube`))
  ;[1 1 1] Изменение материала при ударе
  (if (== NewHealth 2)
    (`PrimitiveComponent.SetMaterial` _cube 0 "/Game/Actors/Materials/Yellow.Yellow")
    (`KismetSystemLibrary.PrintString` (`KismetSystemLibrary.GetDisplayName` _cube) :!label _label)
    (elif (== NewHealth 1)
      (`PrimitiveComponent.SetMaterial` _cube 0 "/Game/Actors/Materials/Green.Green")
      (goto _label))))

(fn `Spawn_Bonuse`
  ;[1 1 1] Спавн бонуса
  (`self.K2_DestroyActor`)
  (if (`KismetMathLibrary.RandomBoolWithWeight` 0.25)
    (`|SpawnActorFromClass` "/Game/Actors/Bonuses/BP_BonuseWithEffect.BP_BonuseWithEffect_C" (`self.GetTransform`) "Undefined" "MultiplyWithRoot" null null)))

(fn `UserConstructionScript`)