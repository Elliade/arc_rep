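; BP_BonuseBall is a bonus ball actor that bounces around the level until it reaches a kill volume.
; Each Tick it makes a swept move along Direction at Velocity, scaled by delta time.
; On a blocking hit, GetReflectionVector recomputes Direction from the X and Y of the hit normal.
; Overlapping a KillZVolume destroys the ball.
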(event `self.ReceiveTick`
  (params (DeltaSeconds :type "Float (single-precision)"))
  ;[1 1 1] Движение шарика
  (bind _sweephitresult (`self.K2_AddActorWorldOffset` (* (* (`self.Direction`) (`self.Velocity`)) DeltaSeconds) true))
  (bind (_bblockinghit _binitialoverlap _time _distance _location _impactpoint _normal) (`GameplayStatics.BreakHitResult` _sweephitresult))
  (if _bblockinghit
    (set `self.Direction` (`KismetMathLibrary.GetReflectionVector` (`self.Direction`) (`KismetMathLibrary.MakeVector` (.x _normal) (.y _normal))))))

(event `self.ReceiveActorBeginOverlap`
  (params (OtherActor :type "Actor Object Reference"))
  ;[1 1 1] Шарик уничтожается
  (cast `KillZVolume` OtherActor)
  (`self.K2_DestroyActor`))

(fn `UserConstructionScript`)