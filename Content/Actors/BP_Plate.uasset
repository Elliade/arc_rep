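; BP_Plate is the player's paddle pawn, moved along X in fixed swept steps by the Movement input axis and spawning a BP_Ball at its Sphere on BeginPlay.
; It binds to the ball's death and to its health component's update and death events.
; Its handlers subtract health and respawn the ball, shrink the Cube by the new-to-old health ratio, and destroy the pawn.
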(event `self.ReceiveBeginPlay`
  ;[1 1 1] Старт игры
  (`self.Binds`)
  (`self.SpawnBall`))

(event `InputAxis|Movement`
  (params (AxisValue :type "Float (single-precision)"))
  ;[1 1 1] Движение пешки
  (if (> AxisValue 0.0)
    (`self.K2_AddActorWorldOffset` (-50.0 0.0 0.0) true)))

(event `InputAxis|Movement`
  (params (AxisValue :type "Float (single-precision)"))
  ;[1 1 1] Движение пешки
  (if (< AxisValue 0.0)
    (`self.K2_AddActorWorldOffset` (50.0 0.0 0.0) true)))

(fn `Binds`
  (bind _bp_healthcomponent (`self.BP_HealthComponent`))
  (add `/Game/Actors/ActorComponents/BP_HealthComponent.OnHealthUpdate` _bp_healthcomponent (`|CreateDelegate` :!event `DescreasePawnScale`))
  (add `/Game/Actors/ActorComponents/BP_HealthComponent.OnDeath` _bp_healthcomponent (`|CreateDelegate` :!event `Destroy_Pawn`)))

(fn `DescreasePawnScale`
  (params (OldHealth :type Integer) (NewHealth :type Integer))
  (bind _cube (`self.Cube`))
  ;[1 1 1] Изменение размера пешки
  (`SceneComponent.SetWorldScale3D` _cube (* (/ NewHealth OldHealth) (`SceneComponent.K2_GetComponentScale` _cube))))

(fn `Destroy_Pawn`
  ;[1 1 1] Уничтожение пешки
  (`self.K2_DestroyActor`))

(fn `RespawnBall`
  ;[1 1 1] Респавн основного мячика
  (`/Game/Actors/ActorComponents/BP_HealthComponent.Sub` (`self.BP_HealthComponent`))
  (`self.SpawnBall`))

(fn `SpawnBall`
  ;[1 1 1] Спавн основного мячика
  (bind _returnvalue (`|SpawnActorFromClass` "/Game/Actors/BP_Ball.BP_Ball_C" (`KismetMathLibrary.MakeTransform` (`SceneComponent.K2_GetComponentLocation` (`self.Sphere`))) "AlwaysSpawn" "MultiplyWithRoot" null null))
  (bind _output_get (set `self.BP_Ball` _returnvalue))
  (add `/Game/Actors/BP_Ball.OnDead` _output_get (`|CreateDelegate` :!event `RespawnBall`))
  (return))

(fn `UserConstructionScript`)